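; Train car that rides the spline of the BP_Train_Track found in the level.
; Tick advances front and rear wheel distances by Speed, snaps both wheel sets to the spline, spins tyres and centres the body between them, aimed at the front.
; CheckLoop handles distances passing either spline end and stops the car unless Loop is set.
; Start and speed changes cascade to AttachWagon through messages, with start delayed briefly per car.
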(event EventBeginPlay
  (CallFunction|CacheTrainTrack)
  (CallFunction|GetWheelDistance))

(event EventStartTrain
  (bind _attach_wagon (Variables|Default|GetAttach_Wagon))
  ;[0 0 0] Start Moving Wagon After Delay
  (Variables|Default|SetbMove? true)
  (Utilities|FlowControl|Delay 0.1)
  (Utilities|IsValid _attach_wagon
    (:Is%20Valid
      (Class|ITrain|StartTrain(Message) _attach_wagon))))

(event EventTick
  (params (DeltaSeconds :type Float%20%28single-precision%29))
  (Variables|Default|SetDelta%20Seconds DeltaSeconds)
  (if (Variables|Default|GetbMove?)
    (CallFunction|UpdateWheelDistance)
    (CallFunction|MoveWheel)
    (CallFunction|RotateWheel)
    (CallFunction|MoveTrain)
    (Utilities|FlowControl|Sequence
      (:then_0
        (bind _distanceout (CallFunction|CheckLoop (Variables|Default|GetFront_Wheel_Disatnce)))
        (Variables|Default|SetFront_Wheel_Disatnce _distanceout))
      (:then_1
        (bind _distanceout_2 (CallFunction|CheckLoop (Variables|Default|GetRear_Wheel_Distance)))
        (Variables|Default|SetRear_Wheel_Distance _distanceout_2)))))

(event EventUpdateSpeed
  (params (New_Speed :type Float%20%28double-precision%29))
  (bind _attach_wagon (Variables|Default|GetAttach_Wagon))
  ;[0 0 0] Update Speed
  (Variables|Default|SetSpeed New_Speed)
  (Utilities|IsValid _attach_wagon
    (:Is%20Valid
      (Class|ITrain|UpdateSpeed(Message) _attach_wagon New_Speed))))

(fn ConstructionScript)

(fn CacheTrainTrack
  (bind _returnvalue (Actor|GetActorOfClass "/Game/Game_Programming/Blueprints/Train_Track_N_Train/BP_Train_Track.BP_Train_Track_C"))
  (Variables|Default|SetTrain_Track _returnvalue))

(fn GetWheelDistance
  (bind _train_track (Variables|Default|GetTrain_Track))
  (bind _train_track_2 (Variables|Default|GetTrain_Track))
  (bind _spline (Variables|/Game/Game_Programming/Blueprints/Train_Track_N_Train/BP_Train_Track.BP_Train_Track_C|GetSpline _train_track))
  (bind _spline_2 (Variables|/Game/Game_Programming/Blueprints/Train_Track_N_Train/BP_Train_Track.BP_Train_Track_C|GetSpline _train_track_2))
  (Variables|Default|SetRear_Wheel_Distance (Class|SplineComponent|GetDistanceAlongSplineatSplineInputKey _spline_2 (Class|SplineComponent|FindInputKeyClosesttoWorldLocation _spline_2 (Transformation|GetWorldLocation (Variables|Default|GetBackTyreP)))))
  (Variables|Default|SetFront_Wheel_Disatnce (Class|SplineComponent|GetDistanceAlongSplineatSplineInputKey _spline (Class|SplineComponent|FindInputKeyClosesttoWorldLocation _spline (Transformation|GetWorldLocation (Variables|Default|GetFrontTyreP))))))

(fn UpdateWheelDistance
  (bind _delta_seconds (Variables|Default|GetDelta%20Seconds))
  (bind _speed (Variables|Default|GetSpeed))
  (bind _returnvalue (* _delta_seconds _speed))
  (Variables|Default|SetFront_Wheel_Disatnce (+ (Variables|Default|GetFront_Wheel_Disatnce) _returnvalue))
  (Variables|Default|SetRear_Wheel_Distance (+ (Variables|Default|GetRear_Wheel_Distance) _returnvalue)))

(fn MoveWheel
  (bind _train_track (Variables|Default|GetTrain_Track))
  (bind _rear_wheel_distance (Variables|Default|GetRear_Wheel_Distance))
  (bind _train_track_2 (Variables|Default|GetTrain_Track))
  (bind _front_wheel_disatnce (Variables|Default|GetFront_Wheel_Disatnce))
  (bind _spline (Variables|/Game/Game_Programming/Blueprints/Train_Track_N_Train/BP_Train_Track.BP_Train_Track_C|GetSpline _train_track))
  (bind _spline_2 (Variables|/Game/Game_Programming/Blueprints/Train_Track_N_Train/BP_Train_Track.BP_Train_Track_C|GetSpline _train_track_2))
  (bind _returnvalue (Spline|GetTransformatDistanceAlongSpline _spline_2 _rear_wheel_distance "World" false))
  (bind _returnvalue_2 (Spline|GetTransformatDistanceAlongSpline _spline _front_wheel_disatnce "World" false))
  ;[1 1 1] Front Wheel
  (Transformation|SetWorldTransform (Variables|Default|GetFrontTyreP) (Math|Transform|MakeTransform (.location _returnvalue_2) (.rotation _returnvalue_2) "1.000000,1.000000,1.000000") false false)
  ;[1 1 1] Back Wheel
  (Transformation|SetWorldTransform (Variables|Default|GetBackTyreP) (Math|Transform|MakeTransform (.location _returnvalue) (.rotation _returnvalue) "1.000000,1.000000,1.000000") false false))

(fn RotateWheel
  (bind _speed (Variables|Default|GetSpeed))
  (if (!= _speed 0.0)
    (Transformation|AddLocalRotation (Variables|Default|GetTrain_Engine_Tyre_1) (Math|Rotator|MakeRotator 0.0 (* (/ _speed 2e+02) -1.0) 0.0) false false)))

(fn MoveTrain
  (bind _backtyrep (Variables|Default|GetBackTyreP))
  (bind _fronttyrep (Variables|Default|GetFrontTyreP))
  (bind _relativelocation (Variables|/Script/Engine.SceneComponent|GetRelativeLocation _fronttyrep))
  (bind _relativelocation_2 (Variables|/Script/Engine.SceneComponent|GetRelativeLocation _backtyrep))
  (bind _returnvalue (+ _relativelocation_2 _relativelocation))
  (bind _returnvalue_2 (* _returnvalue 0.5))
  (Transformation|SetRelativeTransform (Variables|Default|GetBodyP) (Math|Transform|MakeTransform _returnvalue_2 (Math|Rotator|FindLookatRotation _returnvalue_2 _relativelocation) "1.000000,1.000000,1.000000") false false))

(fn CheckLoop
  (params (Distance :type Float%20%28double-precision%29))
  (if (>= Distance (Spline|GetSplineLength (Variables|/Game/Game_Programming/Blueprints/Train_Track_N_Train/BP_Train_Track.BP_Train_Track_C|GetSpline (Variables|Default|GetTrain_Track))))
    (LocalVariables|SetCalDistance 0.0)
    (elif (< Distance 0.0)
      (LocalVariables|SetCalDistance (- (Spline|GetSplineLength (Variables|/Game/Game_Programming/Blueprints/Train_Track_N_Train/BP_Train_Track.BP_Train_Track_C|GetSpline (Variables|Default|GetTrain_Track))) Distance))
      (else
        (return Distance))))
  (if (Variables|Default|GetbLoop?)
    _
    (else
      (Variables|Default|SetSpeed 0.0)
      (Variables|Default|SetbMove? false)))
  (return (LocalVariables|GetCalDistance)))

(fn OnRepBMove?)